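; BP_MyTreasureItem is a treasure item actor with a box collider, intended as a player pickup that updates score.
; End overlap checks for the player character and clears the in-collider flag.
; Begin overlap is unwired, so the logic that sets the flag, casts the game mode and destroys the actor never runs.
; The game mode's score update call is also disconnected, separate from that pickup chain.
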(event `self.BoxCollider.OnComponentBeginOverlap`
  (params (OverlappedComponent :type "PrimitiveComponent Object Reference") (OtherActor :type "Actor Object Reference") (OtherComp :type "PrimitiveComponent Object Reference") (OtherBodyIndex :type Integer) (bFromSweep :type Boolean) (SweepResult :type "HitResult Structure (by ref)"))
  ;[1 1 1] If Player overlaps with item then show prompt and pick up item
)

(event `self.BoxCollider.OnComponentEndOverlap`
  (params (OverlappedComponent :type "PrimitiveComponent Object Reference") (OtherActor :type "Actor Object Reference") (OtherComp :type "PrimitiveComponent Object Reference") (OtherBodyIndex :type Integer))
  ;[1 1 1] If Player exits colider remove prompt
  (if (`.ReturnValue` (`self.CheckPlayerCharacter` OtherActor))
    (`self.SetIsInCollider` false)))

(fn `UserConstructionScript`)