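; Game mode Blueprint for an item-collection game, built to track score against a total and handle win and game-over.
; Binding graphs route a score-update event to increment the score, check for a win and refresh the score text, and bind a game-end event.
; BeginPlay is empty, and the setup chain (item total, load, widget, bindings) is unwired.
; The game-end event is also empty, leaving GameOver disconnected.
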(event `NotifyGameEnd_Event`)

(event `Increase Score`
  (`self.IncrementScore` null)
  (`self.WinGame`)
  (set `TextBlock.Text` (`|FormatText` "Score:{score}/{total}" (`self.score`) _) (`self.txtScore`)))

(event `self.ReceiveBeginPlay`)

(fn `UserConstructionScript`)