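; Player controller Blueprint that routes player input for movement, camera, jump and sprint.
; Axis and action events forward to Call functions, with Sprint using the same call on press and release.
; The L key casts the game mode to TreasureHunterInCppGameModeBase and calls LoadDLC.
; The P key drives SetGamePaused from a FlipFlop to toggle pause.
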(event `InputAxis|MoveForward`
  (params (AxisValue :type "Float (single-precision)"))
  ;[1 1 1] Movement/ WASD Controls
  (`self.CallMoveForward` AxisValue))

(event `InputAction|Jump`
  (params (Key :type "Key Structure"))
  ;[1 1 1] Jump Actions
  (:`Pressed`
    (`self.CallJump`))
  (:`Released`
    (`self.CallJumpEnd`)))

(event `InputAxis|MoveRight`
  (params (AxisValue :type "Float (single-precision)"))
  ;[1 1 1] Movement/ WASD Controls
  (`self.CallMoveRight` AxisValue))

(event `InputAxis|Turn`
  (params (AxisValue :type "Float (single-precision)"))
  ;[1 1 1] Camera/Mouse Controls
  (`self.CallTurn` AxisValue))

(event `InputAction|Sprint`
  (params (Key :type "Key Structure"))
  ;[1 1 1] Sprint Action
  (:`Pressed`
    (`self.CallSprint`))
  (:`Released`
    (`self.CallSprint`)))

(event `InputAxis|LookUp`
  (params (AxisValue :type "Float (single-precision)"))
  ;[1 1 1] Camera/Mouse Controls
  (`self.CallLookUp` AxisValue))

(event `Key|L` :paused true
  (params (Key :type "Key Structure"))
  (:`Pressed`
    (bind _astreasure_hunter_in_cpp_game_mode_base (cast `TreasureHunterInCppGameModeBase` (`GameplayStatics.GetGameMode`)))
    (`TreasureHunterInCppGameModeBase.LoadDLC` _astreasure_hunter_in_cpp_game_mode_base)))

(event `Key|P` :paused true
  (params (Key :type "Key Structure"))
  (:`Pressed`
    (bind _isa (`/Engine/EditorBlueprintResources/StandardMacros.FlipFlop`)
      (:`A`
        _)
      (:`B`
        _))
    (`GameplayStatics.SetGamePaused` _isa)))

(fn `UserConstructionScript`)